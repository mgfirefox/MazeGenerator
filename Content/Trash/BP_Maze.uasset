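; BP_Maze is a procedural grid maze generator meant to lay out floor tiles as mesh instances.
; GenerateMaze runs a seeded, randomized depth-first carve, with AddNeighborLocation recursively stepping two cells to unvisited spots and recording dead ends.
; Backtrack pops pending cells and moves the bridge cells between steps into the path set.
; The construction-script code that calls GenerateMaze and spawns Floor instances is disconnected, so nothing currently builds.
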(event EventBeginPlay)

(event Collision|EventActorBeginOverlap
  (params (OtherActor :type Actor%20Object%20Reference)))

(event EventTick
  (params (DeltaSeconds :type Float%20%28single-precision%29)))

(fn ConstructionScript)

(fn GenerateMaze
  (params (Seed :type Integer) (Size :type Int%20Point%20Structure))
  (Math|Random|SetRandomStreamSeed (LocalVariables|GetRandomStream) Seed)
  (LocalVariables|SetMazeSize Size)
  (bind _output_get (LocalVariables|SetStartingLocation (Utilities|GetRandomLocation (LocalVariables|GetMazeSize) (LocalVariables|GetRandomStream))))
  (LocalVariables|SetCurrentLocation _output_get)
  (CallFunction|AddNeighborLocation (LocalVariables|GetMazeSize) (LocalVariables|GetRandomStream) (LocalVariables|GetCurrentLocation) (LocalVariables|GetPathTiles) (LocalVariables|GetBridgeTiles) (LocalVariables|GetToCheck) (LocalVariables|GetEndPaths) :!label _label)
  (if (> (Utilities|Set|Length (LocalVariables|GetPathTiles)) 0)
    (CallFunction|Backtrack (LocalVariables|GetCurrentLocation) (LocalVariables|GetToCheck) (LocalVariables|GetPathTiles) (LocalVariables|GetBridgeTiles))
    (goto _label)
    (else
      (return (LocalVariables|GetPathTiles) (LocalVariables|GetEndPaths)))))

(fn AddNeighborLocation
  (params (Size :type Int%20Point%20Structure%20%28by%20ref%29) (RandomStream :type Random%20Stream%20Structure%20%28by%20ref%29) (CurrentLocation :type Int%20Point%20Structure%20%28by%20ref%29) (PathTiles :type Set%20of%20Int%20Point%20Structures) (BridgeTiles :type Set%20of%20Int%20Point%20Structures) (ToCheck :type Set%20of%20Int%20Point%20Structures) (EndPaths :type Set%20of%20Int%20Point%20Structures))
  (LocalVariables|SetNeighborIndex (Math|Random|RandomIntegerinRangefromStream RandomStream 0 3))
  (bind _floor (CallFunction|GetNeighborandBridge1 CurrentLocation (LocalVariables|GetNeighborIndex)))
  (if (Utilities|IsValidLocation _floor Size PathTiles BridgeTiles) :!label _label
    (bind (_floor_2 _bridge) (CallFunction|GetNeighborandBridge1 CurrentLocation (LocalVariables|GetNeighborIndex)))
    (Utilities|Set|Add PathTiles _floor_2)
    (Utilities|Set|Add BridgeTiles _bridge)
    (Utilities|Set|Add ToCheck _floor_2)
    (CallFunction|AddNeighborLocation Size RandomStream _floor_2 PathTiles BridgeTiles ToCheck EndPaths)
    (else
      (Utilities|CustomDoN 4
        (:Exit
          (LocalVariables|SetNeighborIndex (Math|Integer|SelectInt 0 (+ (LocalVariables|GetNeighborIndex) 1) (> (+ (LocalVariables|GetNeighborIndex) 1) 3)))
          (goto _label))
        (:OverNIndex
          (bind _count (CallFunction|GetNeighborCount CurrentLocation PathTiles))
          (if (== _count 1)
            (Utilities|Set|Add EndPaths CurrentLocation)))))))

(fn GetNeighborLocation1
  (params (Target :type Int%20Point%20Structure) (Distance :type Integer))
  (bind _returnvalue (* Distance -1))
  (return (Utilities|Array|MakeArray (+ Target (Utilities|Struct|MakeIntPoint Distance 0)) (+ Target (Utilities|Struct|MakeIntPoint 0 Distance)) (+ Target (Utilities|Struct|MakeIntPoint _returnvalue 0)) (+ Target (Utilities|Struct|MakeIntPoint 0 _returnvalue)))))

(fn GetNeighborCount
  (params (CurrentLocation :type Int%20Point%20Structure%20%28by%20ref%29) (PathTiles :type Set%20of%20Int%20Point%20Structures))
  (bind _neighbors (CallFunction|GetNeighborLocation1 CurrentLocation 1))
  (for _array_element _neighbors
    (if (Utilities|Set|Contains PathTiles _array_element)
      (Math|Integer|IncrementInt (LocalVariables|GetCounter))))
  (return (LocalVariables|GetCounter)))

(fn Backtrack
  (params (CurrentTile :type Int%20Point%20Structure) (ToCheck :type Set%20of%20Int%20Point%20Structures) (PathTiles :type Set%20of%20Int%20Point%20Structures) (BridgeTiles :type Set%20of%20Int%20Point%20Structures))
  (bind _result (Utilities|Set|ToArray ToCheck))
  (|SetBy-RefVar CurrentTile (Utilities|Array|Get(acopy) _result (Utilities|Array|LastIndex _result)))
  (Utilities|Set|Remove ToCheck (Utilities|Array|Get(acopy) _result (Utilities|Array|LastIndex _result)))
  (bind _result_2 (Utilities|Set|ToArray BridgeTiles))
  (Utilities|Set|Add PathTiles (Utilities|Array|Get(acopy) _result_2 (Utilities|Array|LastIndex _result_2)))
  (Utilities|Set|Remove BridgeTiles (Utilities|Array|Get(acopy) _result_2 (Utilities|Array|LastIndex _result_2))))

(fn GetNeighborandBridge1
  (params (Target :type Int%20Point%20Structure) (Index :type Integer))
  (bind _neighbors (CallFunction|GetNeighborLocation1 Target 2))
  (bind _neighbors_2 (CallFunction|GetNeighborLocation1 Target 1))
  (return (Utilities|Array|Get(acopy) _neighbors Index) (Utilities|Array|Get(acopy) _neighbors_2 Index)))